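; AI controller for enemies with an AI Perception component, currently inert in its graphs: Tick, BeginPlay and the perception update event are all empty.
; Disconnected draft nodes would run BT_EnemyAI, store a sensed player in the misspelled "PayerCharacter" Blackboard key or clear it, and record ammo spawn points.
; Other unwired fragments experiment with moving directly to actors, including the first pickup spawn point found.
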(event OnTargetPerceptionUpdated(AIPerceptionComponent)
  (params (Actor :type Actor%20Object%20Reference) (Stimulus :type AI%20Stimulus%20Structure)))

(event EventTick
  (params (DeltaSeconds :type Float%20%28single-precision%29)))

(event EventBeginPlay)

(fn ConstructionScript)